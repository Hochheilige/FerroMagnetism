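; BP_CrystallParent is a crystal actor that awards coins when hit, named as a parent for crystal variants.
; The HitBPI event destroys the actor, plays a pitched-down Ding sound and adds its Coin value to CoinCollected on GI_Game.
; It then spawns the P_CrystallDrop particle effect at its location, uniformly sized by its Scale variable.
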(event `/Game/Blueprints/BPI_Hittable.HitBPI`
  (bind _scale (`self.scale`))
  (`self.K2_DestroyActor`)
  (`GameplayStatics.PlaySound2D` "/Game/Sound/ding.ding" 1.0 0.8 0.0 null null)
  (bind _asgi_game (cast `/Game/Blueprints/game/GI_Game` (`GameplayStatics.GetGameInstance`)))
  (set `/Game/Blueprints/game/GI_Game.CoinCollected` (+ (`/Game/Blueprints/game/GI_Game.CoinCollected` _asgi_game) (`self.Coin`)) _asgi_game)
  (`GameplayStatics.SpawnEmitterAtLocation` "/Game/fx/P_CrystallDrop.P_CrystallDrop" (`self.K2_GetActorLocation`) (struct) (`KismetMathLibrary.MakeVector` _scale _scale _scale)))

(fn `UserConstructionScript`)