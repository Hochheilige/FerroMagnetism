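; EnemyParent is an enemy Blueprint, apparently a base class, that dies when struck by a ParryBullet.
; A capsule hit that casts to ParryBullet plays Ding and calls Dead, which hides the mesh and plays Ding again.
; Dead then drops global time dilation for a slow-motion hit-stop, restores it after a brief Delay that the dilation stretches, and destroys the actor.
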(event `dead`
  (`SceneComponent.SetVisibility` (`self.StaticMesh`) false true)
  (`GameplayStatics.PlaySound2D` "/Game/Sound/ding.ding" 0.8 1.0 0.0 null null)
  (`GameplayStatics.SetGlobalTimeDilation` 0.02)
  (`KismetSystemLibrary.Delay` 0.02)
  (`GameplayStatics.SetGlobalTimeDilation` 1.0)
  (`self.K2_DestroyActor`))

(event `self.CapsuleComponent.OnComponentHit`
  (params (HitComponent :type "PrimitiveComponent Object Reference") (OtherActor :type "Actor Object Reference") (OtherComp :type "PrimitiveComponent Object Reference") (NormalImpulse :type "Vector Structure") (Hit :type "HitResult Structure (by ref)"))
  (cast `/Game/Blueprints/ParryBullet` OtherActor)
  (`GameplayStatics.PlaySound2D` "/Game/Sound/ding.ding" 1.0 1.0 0.0 null null)
  (`self.dead`))

(fn `UserConstructionScript`)