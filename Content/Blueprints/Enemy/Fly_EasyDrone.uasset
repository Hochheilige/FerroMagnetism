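; Flying easy drone enemy that, while alive, turns to face the player within range and shoots when the player is close.
; Tick smooths the rotation and, at shorter range, runs a random Delay that paces attacks before a line trace confirms sight of the player.
; Shot plays a charge sound and a timeline that drives spotlight intensity and, on its event track, spawns a bullet with a firing sound.
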(event `self.ReceiveBeginPlay`)

(event `self.ReceiveTick`
  (params (DeltaSeconds :type "Float (single-precision)"))
  (if (`self.isDead?`)
    _
    (elif (not (> (`KismetMathLibrary.Vector_Distance` (`self.K2_GetActorLocation`) (`self.K2_GetActorLocation` (`GameplayStatics.GetPlayerCharacter` 0))) 15000.0))
      (`self.K2_SetActorRotation` (`KismetMathLibrary.RInterpTo` (`self.K2_GetActorRotation`) (`KismetMathLibrary.Conv_VectorToRotator` (`KismetMathLibrary.GetDirectionUnitVector` (`self.K2_GetActorLocation`) (`self.K2_GetActorLocation` (`GameplayStatics.GetPlayerCharacter` 0)))) (`GameplayStatics.GetWorldDeltaSeconds`) 5.0))
      (if (< (`KismetMathLibrary.Vector_Distance` (`self.K2_GetActorLocation`) (`self.K2_GetActorLocation` (`GameplayStatics.GetPlayerCharacter` 0))) 2000.0)
        (`KismetSystemLibrary.Delay` (`KismetMathLibrary.RandomFloatInRange` 1.0 5.0))
        (bind _outhit (`KismetSystemLibrary.LineTraceSingleForObjects` (`self.K2_GetActorLocation`) (`self.K2_GetActorLocation` (`GameplayStatics.GetPlayerCharacter` 0)) (`|MakeArray` "ObjectTypeQuery1" "ObjectTypeQuery3" :!type "EObjectTypeQuery Enum")))
        (cast `/Game/Blueprints/BP_PlayerCharacterED` (`.HitActor` (`GameplayStatics.BreakHitResult` _outhit)))
        (`self.Shot`)))))

(event `Shot`
  (bind _scene1 (`self.Scene1`))
  (bind (_returnvalue_location _returnvalue_rotation) (`KismetMathLibrary.BreakTransform` (`SceneComponent.K2_GetComponentToWorld` _scene1)))
  (`GameplayStatics.SpawnSoundAtLocation` "/Game/Sound/charge.charge" (`SceneComponent.K2_GetComponentLocation` _scene1) (struct) 3.0 1.0 0.0 "/Game/Sound/SA_Long.SA_Long" null)
  (bind (_direction _newtrack_0) (`Timeline|Timeline_0` :!via `PlayFromStart`)
    (:`Update`
      (`LightComponent.SetIntensity` (`self.SpotLight`) (* _newtrack_0 5000.0)))
    (:`NewTrack_1`
      (`|SpawnActorFromClass` "/Game/Blueprints/EnemyBullet.EnemyBullet_C" (`KismetMathLibrary.MakeTransform` _returnvalue_location _returnvalue_rotation) "Undefined" "OverrideRootScale" null null)
      (`GameplayStatics.SpawnSoundAtLocation` "/Game/Sound/enemyshot.enemyshot" (`SceneComponent.K2_GetComponentLocation` (`self.StaticMesh`)) (struct) 0.6 1.0 0.0 "/Game/Sound/SA_Long.SA_Long" null))))

(fn `UserConstructionScript`
  (`parent.UserConstructionScript`))