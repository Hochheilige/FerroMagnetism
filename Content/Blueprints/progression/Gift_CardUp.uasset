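; Progression gift Blueprint that gives the player one card pickup from the deck.
; On DoAction, it casts the player pawn to PlayerCharacterEd and calls PickupCardFromDeck for one card.
; Before that, if IntoDeck and DiscardDeck together hold one card or fewer, it adds a Card_Shot to the discard pile.
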(event `self.DoAction`
  (bind _asplayer_character_ed (cast `/Game/Actors/PlayerCharacterEd` (`GameplayStatics.GetPlayerPawn` 0)))
  (if (<= (+ (`KismetArrayLibrary.Array_Length` (`/Game/Actors/PlayerCharacterEd.IntoDeck` _asplayer_character_ed)) (`KismetArrayLibrary.Array_Length` (`/Game/Actors/PlayerCharacterEd.DiscardDeck` _asplayer_character_ed))) 1)
    (`KismetArrayLibrary.Array_Add` (`/Game/Actors/PlayerCharacterEd.DiscardDeck` _asplayer_character_ed) "/Game/Actors/HandAndCards/Card_Shot.Card_Shot_C"))
  (`/Game/Actors/PlayerCharacterEd.Pickup Card From Deck` _asplayer_character_ed 1))

(fn `UserConstructionScript`
  (`parent.UserConstructionScript`))