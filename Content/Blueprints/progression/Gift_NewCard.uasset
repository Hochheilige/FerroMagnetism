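; Gift pickup that adds a random card to the player's discard deck when its action runs.
; On BeginPlay it picks one card class from a fixed pool of attack, trap, step and other cards.
; It briefly spawns that card far below the origin to copy its face material onto the gift's mesh, then destroys it.
; DoAction appends the chosen class to PlayerCharacterEd's DiscardDeck.
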(event `self.ReceiveBeginPlay`
  (`parent.ReceiveBeginPlay`)
  (set `self.CurrentCard` (`KismetArrayLibrary.Array_Random` (`|MakeArray` "/Game/Actors/HandAndCards/Card_Melee.Card_Melee_C" "/Game/Actors/HandAndCards/Card_Rage.Card_Rage_C" "/Game/Actors/HandAndCards/Card_Trap.Card_Trap_C" "/Game/Actors/HandAndCards/Card_Shot.Card_Shot_C" "/Game/Actors/HandAndCards/Card_StepLeft.Card_StepLeft_C" "/Game/Actors/HandAndCards/Card_StepRight.Card_StepRight_C" "/Game/Actors/HandAndCards/Card_Wind.Card_Wind_C" :!type "/Game/Actors/HandAndCards/CardBaseParent Class Reference")))
  (bind _returnvalue (`|SpawnActorFromClass` (`self.CurrentCard`) (`KismetMathLibrary.MakeTransform` (0.0 0.0 -2000.0)) "Undefined" "OverrideRootScale" null false 0 null))
  (bind _output_get (set `self.TempCard` _returnvalue))
  (`PrimitiveComponent.SetMaterial` (`self.StaticMesh`) 2 (`PrimitiveComponent.GetMaterial` (`/Game/Actors/HandAndCards/CardBaseParent.StaticMesh` _output_get) 2))
  (`self.K2_DestroyActor` _output_get))

(event `self.DoAction`
  (bind _asplayer_character_ed (cast `/Game/Actors/PlayerCharacterEd` (`GameplayStatics.GetPlayerPawn` 0)))
  (`KismetArrayLibrary.Array_Add` (`/Game/Actors/PlayerCharacterEd.DiscardDeck` _asplayer_character_ed) (`self.CurrentCard`)))

(fn `UserConstructionScript`
  (`parent.UserConstructionScript`))