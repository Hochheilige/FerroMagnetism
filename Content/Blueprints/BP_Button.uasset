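; BP_Button is a toggle button that flips its pressed state when hit and signals linked actors.
; Each HitBPI event plays or reverses a timeline that slides the Button mesh along its local X axis.
; It then swaps the mesh between blue for pressed and red for released.
; Every entry in LinkedActors receives SignalInMessage when pressed and SignalOutMessage when released.
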(event `/Game/Blueprints/BPI_Hittable.HitBPI`
  (bind _button (`self.button`))
  (`|ExecutionSequence`
    (:`then_0`
      (if (`self.pressed?`)
        (set `self.pressed?` false)
        (bind (_direction _newtrack_0) (`Timeline|Timeline_0` :!via `ReverseFromEnd` :!label _label)
          (:`Update`
            (`SceneComponent.K2_SetRelativeLocation` (`self.button`) (`KismetMathLibrary.VLerp` (0.0 0.0 0.0) (-50.0 0.0 0.0) _newtrack_0) false false)))
        (else
          (set `self.pressed?` true)
          (goto _label :!via `PlayFromStart`))))
    (:`then_1`
      (if (`self.pressed?`)
        (`StaticMeshComponent.SetStaticMesh` _button "/Game/3d/button_blue.button_blue")
        (for _array_element (`self.LinkedActors`)
          (message `/Game/Blueprints/BPI_Tech.Signal_In` _array_element))
        (else
          (`StaticMeshComponent.SetStaticMesh` _button "/Game/3d/button_red.button_red")
          (for _array_element_2 (`self.LinkedActors`)
            (message `/Game/Blueprints/BPI_Tech.Signal_Out` _array_element_2)))))))

(fn `UserConstructionScript`)