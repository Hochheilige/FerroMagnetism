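; Enemy turret actor that snaps to face the player every tick and fires at them when in range.
; A random Delay on Tick paces attacks, then a line trace must hit the player character to trigger Shot.
; Shot plays a charge sound and a Timeline that drives spotlight intensity and spawns the enemy bullet.
; Bullet hits destroy it outright; a separate dead event adds brief slow-motion hit-stop before destruction.
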(event `self.ReceiveTick`
  (params (DeltaSeconds :type "Float (single-precision)"))
  (`self.K2_SetActorRotation` (`KismetMathLibrary.Conv_VectorToRotator` (`KismetMathLibrary.GetDirectionUnitVector` (`self.K2_GetActorLocation`) (`self.K2_GetActorLocation` (`GameplayStatics.GetPlayerCharacter` 0)))))
  (if (< (`KismetMathLibrary.Vector_Distance` (`self.K2_GetActorLocation`) (`self.K2_GetActorLocation` (`GameplayStatics.GetPlayerCharacter` 0))) 2000.0)
    (`KismetSystemLibrary.Delay` (`KismetMathLibrary.RandomFloatInRange` 1.0 5.0))
    (bind _outhit (`KismetSystemLibrary.LineTraceSingleForObjects` (`self.K2_GetActorLocation`) (`self.K2_GetActorLocation` (`GameplayStatics.GetPlayerCharacter` 0)) (`|MakeArray` "ObjectTypeQuery1" "ObjectTypeQuery3" :!type "EObjectTypeQuery Enum")))
    (cast `/Game/Blueprints/BP_PlayerCharacterED` (`.HitActor` (`GameplayStatics.BreakHitResult` _outhit)))
    (`self.Shot`)))

(event `Shot`
  (bind (_returnvalue_location _returnvalue_rotation) (`KismetMathLibrary.BreakTransform` (`SceneComponent.K2_GetComponentToWorld` (`self.Scene`))))
  (`GameplayStatics.SpawnSoundAtLocation` "/Game/Sound/charge.charge" (`SceneComponent.K2_GetComponentLocation` (`self.Sphere`)) (struct) 3.0 1.0 0.0 "/Game/Sound/SA_Long.SA_Long" null)
  (bind (_direction _newtrack_0) (`Timeline|Timeline_0` :!via `PlayFromStart`)
    (:`Update`
      (`LightComponent.SetIntensity` (`self.SpotLight`) (* _newtrack_0 5000.0)))
    (:`NewTrack_1`
      (`|SpawnActorFromClass` "/Game/Blueprints/EnemyBullet.EnemyBullet_C" (`KismetMathLibrary.MakeTransform` _returnvalue_location _returnvalue_rotation) "Undefined" "OverrideRootScale" null null)
      (`GameplayStatics.SpawnSoundAtLocation` "/Game/Sound/enemyshot.enemyshot" (`SceneComponent.K2_GetComponentLocation` (`self.Sphere`)) (struct) 0.6 1.0 0.0 "/Game/Sound/SA_Long.SA_Long" null))))

(event `self.Sphere.OnComponentHit`
  (params (HitComponent :type "PrimitiveComponent Object Reference") (OtherActor :type "Actor Object Reference") (OtherComp :type "PrimitiveComponent Object Reference") (NormalImpulse :type "Vector Structure") (Hit :type "HitResult Structure (by ref)"))
  (cast `/Game/Blueprints/bullet` OtherActor)
  (`GameplayStatics.PlaySound2D` "/Game/Sound/ding.ding" 1.0 1.0 0.0 null null)
  (`self.K2_DestroyActor`))

(event `dead`
  (`SceneComponent.SetVisibility` (`self.Sphere`) false true)
  (`GameplayStatics.PlaySound2D` "/Game/Sound/ding.ding" 0.8 1.0 0.0 null null)
  (`GameplayStatics.SetGlobalTimeDilation` 0.02)
  (`KismetSystemLibrary.Delay` 0.02)
  (`GameplayStatics.SetGlobalTimeDilation` 1.0)
  (`self.K2_DestroyActor`))

(fn `UserConstructionScript`)