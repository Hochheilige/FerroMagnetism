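; EnemyBullet is a parryable enemy projectile that kills the player on hit.
; Its Hit event calls DeathPlayer when the other actor is BP_PlayerCharacterED, and destroys the bullet on any impact.
; The HitBPI event performs the parry, replacing the bullet with a ParryBullet at the same location, aimed along the player camera's forward vector, and playing a pitched-up Ding sound.
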(event `self.ReceiveHit`
  (params (MyComp :type "PrimitiveComponent Object Reference") (Other :type "Actor Object Reference") (OtherComp :type "PrimitiveComponent Object Reference") (bSelfMoved :type Boolean) (HitLocation :type "Vector Structure") (HitNormal :type "Vector Structure") (NormalImpulse :type "Vector Structure") (Hit :type "HitResult Structure (by ref)"))
  (bind _asbp_player_character_ed (cast `/Game/Blueprints/BP_PlayerCharacterED` Other)
    (:`then`
      (`/Game/Blueprints/BP_PlayerCharacterED.DeathPlayer` _asbp_player_character_ed))
    (:`CastFailed`
      _))
  (`self.K2_DestroyActor`))

(event `/Game/Blueprints/BPI_Hittable.HitBPI`
  (bind (_returnvalue_location _returnvalue_rotation _returnvalue_scale) (`KismetMathLibrary.BreakTransform` (`self.GetTransform`)))
  (bind _asbp_player_character_ed (cast `/Game/Blueprints/BP_PlayerCharacterED` (`GameplayStatics.GetPlayerCharacter` 0)))
  (`|SpawnActorFromClass` "/Game/Blueprints/ParryBullet.ParryBullet_C" (`KismetMathLibrary.MakeTransform` _returnvalue_location (`KismetMathLibrary.Conv_VectorToRotator` (`SceneComponent.GetForwardVector` (`/Game/Blueprints/BP_PlayerCharacterED.Camera` _asbp_player_character_ed))) _returnvalue_scale) "Undefined" "OverrideRootScale" null null)
  (`self.K2_DestroyActor`)
  (`GameplayStatics.PlaySound2D` "/Game/Sound/ding.ding" 1.0 2.0 0.0 null null))

(fn `UserConstructionScript`)