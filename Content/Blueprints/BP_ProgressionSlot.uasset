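; BP_ProgressionSlot is an in-world upgrade kiosk that opens the progression menu when hit through a blueprint interface.
; On HitBPI it creates the UI_Progression widget, adds it to the viewport and shows the player's mouse cursor.
; Tick drives a randomly timed Delay that swaps its TextRender between random upgrade taunt lines.
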(event `/Game/Blueprints/BPI_Hittable.HitBPI`
  (bind _returnvalue (`|CreateWidget` "/Game/UI/UI_Progression.UI_Progression_C"))
  (`UserWidget.AddToViewport` _returnvalue 0)
  (set `PlayerController.bShowMouseCursor` true (`GameplayStatics.GetPlayerController` 0)))

(event `self.ReceiveTick`
  (params (DeltaSeconds :type "Float (single-precision)"))
  (`KismetSystemLibrary.Delay` (`KismetMathLibrary.RandomFloatInRange` 0.8 2.0))
  (`TextRenderComponent.K2_SetText` (`self.TextRender`) (`KismetArrayLibrary.Array_Random` (`|MakeArray` "Upgrade!" "..." "Good day \nfor upgrade" "Upgrade \ntime" "do you \nwant \nupgrade?" "I want \nyou \nmoney" :!type "Text"))))

(fn `UserConstructionScript`)